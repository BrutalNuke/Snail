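; Snail actor that moves continuously along its local X axis, with player-adjustable speed.
; Tick offsets the RenderComponent by Speed scaled by delta time.
; Enhanced Input actions add or subtract a SpeedChange step, but only while something overlaps the SpeedUp component, whose begin and end overlap events toggle that permission without filtering the other actor.
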(event `self.ReceiveTick`
  (params (DeltaSeconds :type "Float (single-precision)"))
  (`SceneComponent.K2_AddLocalOffset` (`self.RenderComponent`) (`KismetMathLibrary.MakeVector` (* DeltaSeconds (`self.Speed`))) false false))

(event `EnhancedInput|/Game/Blueprints/IA_SnailSpeedUp`
  (params (ActionValue :type Boolean) (ElapsedSeconds :type "Float (double-precision)") (TriggeredSeconds :type "Float (double-precision)") (InputAction :type "InputAction Object Reference" :default "/Game/Blueprints/IA_SnailSpeedUp.IA_SnailSpeedUp"))
  (:`Triggered`
    (if (`self.SpeedChangeAllowed`)
      (set `self.Speed` (+ (`self.SpeedChange`) (`self.Speed`))))))

(event `EnhancedInput|/Game/Blueprints/IA_SnailSpeedDown`
  (params (ActionValue :type Boolean) (ElapsedSeconds :type "Float (double-precision)") (TriggeredSeconds :type "Float (double-precision)") (InputAction :type "InputAction Object Reference" :default "/Game/Blueprints/IA_SnailSpeedDown.IA_SnailSpeedDown"))
  (:`Triggered`
    (if (`self.SpeedChangeAllowed`)
      (set `self.Speed` (- (`self.Speed`) (`self.SpeedChange`))))))

(event `self.Speed up.OnComponentBeginOverlap`
  (params (OverlappedComponent :type "PrimitiveComponent Object Reference") (OtherActor :type "Actor Object Reference") (OtherComp :type "PrimitiveComponent Object Reference") (OtherBodyIndex :type Integer) (bFromSweep :type Boolean) (SweepResult :type "HitResult Structure (by ref)"))
  (set `self.SpeedChangeAllowed` true))

(event `self.Speed up.OnComponentEndOverlap`
  (params (OverlappedComponent :type "PrimitiveComponent Object Reference") (OtherActor :type "Actor Object Reference") (OtherComp :type "PrimitiveComponent Object Reference") (OtherBodyIndex :type Integer))
  (set `self.SpeedChangeAllowed` false))

(fn `UserConstructionScript`)